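; BP_Debug is a debug helper actor that enables player input to manipulate fish and test throwables.
; Tab cycles the selected FishBase actor, and IJKL and U/O move and rotate it through MoveSelectedFish using tunable multipliers.
; B and R spawn bait and rocks with velocity from ThrowVelocity, while Page Up/Down adjust global time dilation.
; Mouse-wheel throw-speed adjustment and blackboard target assignment are disconnected.
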(event EventBeginPlay
  (Input|EnableInput (Game|GetPlayerController 0))
  (bind _returnvalue (Actor|GetActorOfClass "/Script/FishAi.FishBase"))
  (Variables|Default|SetselectedFish _returnvalue))

(event Input|MouseEvents|MouseWheelAxis
  (params (AxisValue :type Float%20%28single-precision%29))
  ;[1 1 1] throwing
)

(event Input|KeyboardEvents|DebugKeyB
  (params (Key :type Key%20Structure :default "None") (ActionValue :type Input%20Action%20Value%20Structure))
  ;[1 1 1] throwing
  (:Pressed
    (bind _returnvalue (Game|SpawnActorfromClass "/Game/Blueprints/ThrowableObject/BP_Bait1.BP_Bait1_C" (Math|Transform|MakeTransform (Variables|Default|GetBaitSpawnLoc)) "AlwaysSpawn" 0 0))
    (Class|ThrowableObject|SetVelocity _returnvalue (Utilities|ThrowVelocity))))

(event Input|KeyboardEvents|DebugKeyR
  (params (Key :type Key%20Structure :default "None") (ActionValue :type Input%20Action%20Value%20Structure))
  ;[1 1 1] throwing
  (:Pressed
    (bind _returnvalue (Game|SpawnActorfromClass "/Game/Blueprints/ThrowableObject/BP_Rock1.BP_Rock1_C" (Math|Transform|MakeTransform (Variables|Default|GetRockSpawnLoc)) "AlwaysSpawn" 0 0))
    (Class|ThrowableObject|SetVelocity _returnvalue (Utilities|ThrowVelocity))))

(event Input|KeyboardEvents|DebugKeyO
  (params (Key :type Key%20Structure :default "None") (ActionValue :type Input%20Action%20Value%20Structure))
  (:Pressed
    (CallFunction|MoveSelectedFish "0, 0, 0" "0.000000,1.000000,0.000000")))

(event Input|KeyboardEvents|DebugKeyTab
  (params (Key :type Key%20Structure :default "None") (ActionValue :type Input%20Action%20Value%20Structure))
  (bind _selectedfishindex (Variables|Default|GetselectedFishIndex))
  (:Pressed
    (Math|Integer|IncrementInt _selectedfishindex
      (:%20%20
        (bind _outactors (Actor|GetAllActorsOfClass "/Script/FishAi.FishBase"))
        (Variables|Default|SetselectedFish (Utilities|Array|Get(acopy) _outactors (Math|Integer|%(Integer) _selectedfishindex (Utilities|Array|Length _outactors))))))))

(event Input|KeyboardEvents|DebugKeyPageDown
  (params (Key :type Key%20Structure :default "None") (ActionValue :type Input%20Action%20Value%20Structure))
  (:Pressed
    (Utilities|Time|SetGlobalTimeDilation (- (Class|GameplayStatics|GetGlobalTimeDilation) 0.5))))

(event Input|KeyboardEvents|DebugKeyPageUp
  (params (Key :type Key%20Structure :default "None") (ActionValue :type Input%20Action%20Value%20Structure))
  (:Pressed
    (Utilities|Time|SetGlobalTimeDilation (+ (Class|GameplayStatics|GetGlobalTimeDilation) 0.5))))

(event Input|MouseEvents|DebugKeyMouseWheelAxis
  (params (Key :type Key%20Structure :default "None") (ActionValue :type Input%20Action%20Value%20Structure))
  ;[1 1 1] throwing
)

(event Input|KeyboardEvents|DebugKeyT
  (params (Key :type Key%20Structure :default "None") (ActionValue :type Input%20Action%20Value%20Structure)))

(event Input|KeyboardEvents|DebugKeyI
  (params (Key :type Key%20Structure :default "None") (ActionValue :type Input%20Action%20Value%20Structure))
  (:Pressed
    (CallFunction|MoveSelectedFish (Class|KismetMathLibrary|VectorForward) "0, 0, 0")))

(event Input|KeyboardEvents|DebugKeyL
  (params (Key :type Key%20Structure :default "None") (ActionValue :type Input%20Action%20Value%20Structure))
  (:Pressed
    (CallFunction|MoveSelectedFish (Class|KismetMathLibrary|VectorRight) "0, 0, 0")))

(event Input|KeyboardEvents|DebugKeyJ
  (params (Key :type Key%20Structure :default "None") (ActionValue :type Input%20Action%20Value%20Structure))
  (:Pressed
    (CallFunction|MoveSelectedFish (Class|KismetMathLibrary|VectorLeft) "0, 0, 0")))

(event Input|KeyboardEvents|DebugKeyK
  (params (Key :type Key%20Structure :default "None") (ActionValue :type Input%20Action%20Value%20Structure))
  (:Pressed
    (CallFunction|MoveSelectedFish (Class|KismetMathLibrary|VectorBackward) "0, 0, 0")))

(event Input|KeyboardEvents|DebugKeyU
  (params (Key :type Key%20Structure :default "None") (ActionValue :type Input%20Action%20Value%20Structure))
  (:Pressed
    (CallFunction|MoveSelectedFish "0, 0, 0" "0.000000,-1.000000,0.000000")))

(fn ConstructionScript)

(fn MoveSelectedFish
  (params (locDif :type Vector) (rotDif :type Rotator))
  (Class|Actor|AddActorWorldTransform (Variables|Default|GetselectedFish) (Math|Transform|MakeTransform (* locDif (LocalVariables|GetmoveMultiplier)) (* rotDif (LocalVariables|GetrotationMultiplier)) "1.000000,1.000000,1.000000") false false))