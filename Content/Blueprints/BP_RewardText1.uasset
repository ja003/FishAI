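; BP_RewardText1 is a floating actor, named as reward text, that rises while facing the player's camera.
; BeginPlay casts the player character to BP_CPP_MyCharacterZorg1 and caches its Camera.
; Each Tick calls FaceCamera, which applies a look-at rotation toward that camera if valid, then moves the actor up a fixed step, so rise speed depends on frame rate.
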(event EventBeginPlay
  (bind _asbp_cpp_my_character_zorg_1 (Utilities|Casting|CastToBP_CPP_MyCharacterZorg1 (Game|GetPlayerCharacter 0)))
  (Variables|Default|SetCamera (Variables|/Game/Zorg/BP_CPP_MyCharacterZorg1.BP_CPP_MyCharacterZorg1_C|GetCamera _asbp_cpp_my_character_zorg_1)))

(event EventTick
  (params (DeltaSeconds :type Float%20%28single-precision%29))
  (Utilities|FaceCamera)
  (Transformation|SetActorLocation (+ (Transformation|GetActorLocation) "0.000000,0.000000,1.000000") false false))

(fn ConstructionScript)