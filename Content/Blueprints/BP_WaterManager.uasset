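; BP_WaterManager is a water manager Blueprint that records the outline of a referenced water body as 2D points.
; Its SetWaterBounds event loops over the WaterBodyBP spline points, flattens each local-space location to a 2D vector and appends it to WaterBounds.
; It then prints the point count, and nothing in its own graphs calls the event or reads the bounds.
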(event EventBeginPlay)

(event Collision|EventActorBeginOverlap
  (params (OtherActor :type Actor%20Object%20Reference)))

(event EventTick
  (params (DeltaSeconds :type Float%20%28single-precision%29)))

(event EventSetWaterBounds
  (bind _waterbodybp (Variables|Default|GetWaterBodyBP))
  (bind _splinecomp (Variables|/Script/Water.WaterBody|GetSplineComp _waterbodybp))
  (bind _returnvalue (Spline|GetNumberOfSplinePoints _splinecomp))
  (for _index (range 0 (- _returnvalue 1))
    (Utilities|Array|Add (Variables|Default|GetWaterBounds) (Math|Conversions|ToVector2D(Vector) (Spline|GetLocationatSplinePoint _splinecomp _index "Local"))))
  (Development|PrintString (Utilities|String|Append (Utilities|String|ToString(Integer) _returnvalue) " points")))

(fn ConstructionScript)