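; BP_FishCarp is a carp fish whose AI perception reacts to bait and pike by writing to its Blackboard.
; Perceived bait is stored as the Bait object with a matching State change.
; A perceived pike sets another State and a flee Target mirroring the pike's position through the carp, shown with a debug sphere.
; The capsule overlap only casts to bait, as EatBait is left unwired.
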(event OnTargetPerceptionUpdated(AIPerception)
  (params (Actor :type Actor%20Object%20Reference) (Stimulus :type AI%20Stimulus%20Structure))
  (bind _returnvalue (AI|GetBlackboard 0))
  (bind _returnvalue_2 (Transformation|GetActorLocation))
  (bind _returnvalue_3 (AI|GetBlackboard 0))
  (bind _asbp_bait (Utilities|Casting|CastToBP_Bait Actor)
    (:then
      (Development|PrintString "bait")
      (AI|Components|Blackboard|SetValueasObject _returnvalue_3 (Utilities|Name|MakeLiteralName "Bait") _asbp_bait)
      (AI|Components|Blackboard|SetValueasEnum _returnvalue_3 (Utilities|Name|MakeLiteralName "State") (Utilities|Enum|LiteralenumEFishState "NewEnumerator2")))
    (:CastFailed
      (bind _asbp_fish_pike (Utilities|Casting|CastToBP_FishPike Actor))
      (Development|PrintString "pike")
      (AI|Components|Blackboard|SetValueasEnum _returnvalue (Utilities|Name|MakeLiteralName "State") (Utilities|Enum|LiteralenumEFishState "NewEnumerator3"))
      (AI|Components|Blackboard|SetValueasVector _returnvalue (Utilities|Name|MakeLiteralName "Target") (+ _returnvalue_2 (- _returnvalue_2 (Transformation|GetActorLocation _asbp_fish_pike))))
      (Rendering|Debug|DrawDebugSphere (+ _returnvalue_2 (- _returnvalue_2 (Transformation|GetActorLocation _asbp_fish_pike))) 1e+02 12 "(R=1.000000,G=1.000000,B=1.000000,A=1.000000)" 5.0))))

(event OnComponentBeginOverlap(CapsuleComponent)
  (params (OverlappedComponent :type Primitive%20Component%20Object%20Reference) (OtherActor :type Actor%20Object%20Reference) (OtherComp :type Primitive%20Component%20Object%20Reference) (OtherBodyIndex :type Integer) (bFromSweep :type Boolean) (SweepResult :type Hit%20Result%20Structure%20%28by%20ref%29))
  (bind _asbp_bait (Utilities|Casting|CastToBP_Bait OtherActor)))

(event EventBeginPlay
  (|CallParentFunction) ; This node is disabled and will not be called.\nDrag off pins to build functionality.
)

(fn ConstructionScript
  (|CallParentFunction))