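; Pike fish Blueprint that supplies two patrol-style points to its AI and periodically emits noise.
; On BeginPlay it runs the parent logic, writes fixed pointA and pointB vectors to the Blackboard and starts a looping Roar timer.
; Roar reports a limited-range noise event at the pike's location for AI hearing; its debug print and sound playback are disabled.
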(event Custom|Roar
  (bind _returnvalue (Transformation|GetActorLocation))
  (Development|PrintString "roar")
  (Audio|PlaySoundatLocation "/Game/StarterContent/Audio/Collapse01.Collapse01" _returnvalue "0, 0, 0" 1.0 1.0 0.0 0 0 0 0)
  (Class|AISenseHearing|ReportNoiseEvent _returnvalue 1.0 self 5e+02 "None"))

(event EventBeginPlay
  (bind _returnvalue (AI|GetBlackboard 0))
  (|CallParentFunction)
  (AI|Components|Blackboard|SetValueasVector _returnvalue (Utilities|Name|MakeLiteralName "pointA") "180.000000,-230.000000,0.000000")
  (AI|Components|Blackboard|SetValueasVector _returnvalue (Utilities|Name|MakeLiteralName "pointB") "-200.000000,-230.000000,0.000000")
  (Utilities|Time|SetTimerbyEvent (delegate Custom|Roar) 2.0 true))

(fn ConstructionScript
  (|CallParentFunction))