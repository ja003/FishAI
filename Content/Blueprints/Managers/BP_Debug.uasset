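; BP_Debug is a debug manager actor that binds test shortcuts for the fish game on player 0's input.
; Keys step global time dilation, spawn a nav modifier, and spawn and throw bait or rocks.
; Tab cycles the selected FishBase actor, which other keys move or rotate through MoveSelectedFish, while Ctrl+K variants trigger grenade death on one or all fish.
; Mouse-wheel throw-speed adjustment and blackboard targeting are left disconnected.
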(event EventBeginPlay
  (Input|EnableInput (Game|GetPlayerController 0))
  (bind _returnvalue (Actor|GetActorOfClass "/Script/FishAi.FishBase"))
  (Variables|Default|SetselectedFish _returnvalue))

(event Input|MouseEvents|MouseWheelAxis
  (params (AxisValue :type Float%20%28single-precision%29))
  ;[1 1 1] throwing
)

(event Input|KeyboardEvents|DebugKeyB
  (params (Key :type Key%20Structure) (ActionValue :type Input%20Action%20Value%20Structure))
  ;[1 1 1] throwing
  (:Pressed
    (bind _returnvalue (Game|SpawnActorfromClass "/Game/Blueprints/ThrowableObject/BP_Bait.BP_Bait_C" (Math|Transform|MakeTransform (Variables|Default|GetBaitSpawnLoc)) "AlwaysSpawn" 0 0))
    (Class|ThrowableObject|Throw _returnvalue (Utilities|ThrowVelocity))))

(event Input|KeyboardEvents|DebugKeyR
  (params (Key :type Key%20Structure) (ActionValue :type Input%20Action%20Value%20Structure))
  ;[1 1 1] throwing
  (:Pressed
    (bind _returnvalue (Game|SpawnActorfromClass "/Game/Blueprints/ThrowableObject/BP_Rock.BP_Rock_C" (Math|Transform|MakeTransform (Variables|Default|GetRockSpawnLoc)) "AlwaysSpawn" 0 0))
    (Class|ThrowableObject|Throw _returnvalue (Utilities|ThrowVelocity))))

(event Input|KeyboardEvents|DebugKeyO
  (params (Key :type Key%20Structure) (ActionValue :type Input%20Action%20Value%20Structure))
  (:Pressed
    (CallFunction|MoveSelectedFish "0, 0, 0" "0.000000,1.000000,0.000000")))

(event Input|KeyboardEvents|DebugKeyTab
  (params (Key :type Key%20Structure) (ActionValue :type Input%20Action%20Value%20Structure))
  (bind _selectedfishindex (Variables|Default|GetselectedFishIndex))
  (:Pressed
    (Math|Integer|IncrementInt _selectedfishindex
      (:%20%20
        (bind _outactors (Actor|GetAllActorsOfClass "/Script/FishAi.FishBase"))
        (Variables|Default|SetselectedFish (Utilities|Array|Get(acopy) _outactors (Math|Integer|%(Integer) _selectedfishindex (Utilities|Array|Length _outactors))))))))

(event Input|KeyboardEvents|DebugKeyPageDown
  (params (Key :type Key%20Structure) (ActionValue :type Input%20Action%20Value%20Structure))
  (bind _returnvalue (Class|GameplayStatics|GetGlobalTimeDilation))
  (:Pressed
    (Utilities|Time|SetGlobalTimeDilation (- _returnvalue 0.5))
    (Development|PrintString (Utilities|String|Append "time dilation: " (Utilities|String|ToString(Float) _returnvalue)))))

(event Input|KeyboardEvents|DebugKeyCtrlShiftK
  (params (Key :type Key%20Structure) (ActionValue :type Input%20Action%20Value%20Structure))
  (:Pressed
    (bind _outactors (Actor|GetAllActorsOfClass "/Script/FishAi.FishBase"))
    (for _array_element _outactors
      (Class|FishBase|OnKilledbyGrenade _array_element "0.000000,0.000000,100000.000000"))
    (Development|PrintString "debug: kill all fishes")))

(event Input|KeyboardEvents|DebugKeyY
  (params (Key :type Key%20Structure) (ActionValue :type Input%20Action%20Value%20Structure))
  (:Pressed
    (Game|SpawnActorfromClass "/Game/Blueprints/Other/BP_NavModifier.BP_NavModifier_C" (Math|Transform|MakeTransform "355.000000,120.000000,0.000000") "AlwaysSpawn" 0 0)))

(event Input|KeyboardEvents|DebugKeyCtrlK
  (params (Key :type Key%20Structure) (ActionValue :type Input%20Action%20Value%20Structure))
  (:Pressed
    (bind _returnvalue (Actor|GetActorOfClass "/Script/FishAi.FishBase"))
    (Class|FishBase|OnKilledbyGrenade _returnvalue "0.000000,0.000000,100000.000000")))

(event Input|KeyboardEvents|DebugKeyPageUp
  (params (Key :type Key%20Structure) (ActionValue :type Input%20Action%20Value%20Structure))
  (bind _returnvalue (Class|GameplayStatics|GetGlobalTimeDilation))
  (:Pressed
    (Utilities|Time|SetGlobalTimeDilation (+ _returnvalue 0.5))
    (Development|PrintString (Utilities|String|Append "time dilation: " (Utilities|String|ToString(Float) _returnvalue)))))

(event Input|MouseEvents|DebugKeyMouseWheelAxis
  (params (Key :type Key%20Structure) (ActionValue :type Input%20Action%20Value%20Structure))
  ;[1 1 1] throwing
)

(event Input|KeyboardEvents|DebugKeyT
  (params (Key :type Key%20Structure) (ActionValue :type Input%20Action%20Value%20Structure)))

(event Input|KeyboardEvents|DebugKeyI
  (params (Key :type Key%20Structure) (ActionValue :type Input%20Action%20Value%20Structure))
  (:Pressed
    (CallFunction|MoveSelectedFish (Class|KismetMathLibrary|VectorForward) "0, 0, 0")))

(event Input|KeyboardEvents|DebugKeyL
  (params (Key :type Key%20Structure) (ActionValue :type Input%20Action%20Value%20Structure))
  (:Pressed
    (CallFunction|MoveSelectedFish (Class|KismetMathLibrary|VectorRight) "0, 0, 0")))

(event Input|KeyboardEvents|DebugKeyJ
  (params (Key :type Key%20Structure) (ActionValue :type Input%20Action%20Value%20Structure))
  (:Pressed
    (CallFunction|MoveSelectedFish (Class|KismetMathLibrary|VectorLeft) "0, 0, 0")))

(event Input|KeyboardEvents|DebugKeyK
  (params (Key :type Key%20Structure) (ActionValue :type Input%20Action%20Value%20Structure))
  (:Pressed
    (CallFunction|MoveSelectedFish (Class|KismetMathLibrary|VectorBackward) "0, 0, 0")))

(event Input|KeyboardEvents|DebugKeyU
  (params (Key :type Key%20Structure) (ActionValue :type Input%20Action%20Value%20Structure))
  (:Pressed
    (CallFunction|MoveSelectedFish "0, 0, 0" "0.000000,-1.000000,0.000000")))

(fn ConstructionScript)

(fn MoveSelectedFish
  (params (locDif :type Vector) (rotDif :type Rotator))
  (Class|Actor|AddActorWorldTransform (Variables|Default|GetselectedFish) (Math|Transform|MakeTransform (* locDif (LocalVariables|GetmoveMultiplier)) (* rotDif (LocalVariables|GetrotationMultiplier)) "1.000000,1.000000,1.000000") false false))