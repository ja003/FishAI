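; BP_GameManager is a manager Blueprint that shows objective messages for a fish-catching level.
; On BeginPlay it caches the player character BP_CPP_MyCharacterZorg1, creates a WBP_TextMessage widget, adds it to the viewport and sets the starting goal text.
; The OnAllFishesDeadBP event swaps the message to congratulate the player and send them to the next lake.
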(event EventBeginPlay
  (Utilities|FlowControl|Sequence
    (:then_0
      (bind _returnvalue (Actor|GetActorOfClass "/Game/Zorg/BP_CPP_MyCharacterZorg1.BP_CPP_MyCharacterZorg1_C"))
      (bind _output_get (Variables|Default|SetMyCharacter _returnvalue))
      (Utilities|IsValid _output_get))
    (:then_1
      (bind _returnvalue_2 (UserInterface|CreateWidget "/Game/UI/WBP_TextMessage.WBP_TextMessage_C"))
      (Variables|Default|SetUIMessage _returnvalue_2)
      (UserInterface|Viewport|AddtoViewport _returnvalue_2 0)
      (Default|SetText (Variables|Default|GetUIMessage) "Go catch them all!" :!label _label))
    (:then_2
      (goto _label))))

(event EventOnAllFishesDeadBP
  (Default|SetText (Variables|Default|GetUIMessage) "You got them! Go to the next lake!"))

(fn ConstructionScript)