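; Water manager that wraps a water body Blueprint to provide its horizontal bounds and height queries.
; SetWaterBounds stores the world-space spline points as 2D WaterBounds.
; Surface and bottom lookups query the water component at a given location, subtracting depth for the bottom; surface results exclude waves, per the author's note.
; An AllFishesDead event only prints a message, and its binding never runs.
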(event Custom|AllFishesDead
  (Development|PrintString "all fishes dead"))

(event EventBeginPlay)

(event EventSetWaterBounds
  (bind _waterbodybp (Variables|Default|GetWaterBodyBP))
  (bind _splinecomp (Variables|/Script/Water.WaterBody|GetSplineComp _waterbodybp))
  (bind _returnvalue (Spline|GetNumberOfSplinePoints _splinecomp))
  (for _index (range 0 (- _returnvalue 1))
    (Utilities|Array|Add (Variables|Default|GetWaterBounds) (Math|Conversions|ToVector2D(Vector) (Spline|GetLocationatSplinePoint _splinecomp _index "World"))))
  (Development|PrintString (Utilities|String|Append (Utilities|String|ToString(Integer) _returnvalue) " points")))

(fn ConstructionScript)

(fn GetWaterSurfaceLocation
  (params (AtLocation :type Vector :default "0, 0, 0"))
  (bind _waterbodybp (Variables|Default|GetWaterBodyBP))
  (bind _waterbodycomponent (Variables|/Script/Water.WaterBody|GetWaterBodyComponent _waterbodybp))
  (bind (_outwatersurfacelocation _outwatersurfacenormal _outwatervelocity _outwaterdepth) (WaterBody|GetWaterSurfaceInfoatLocation _waterbodycomponent AtLocation true))
  ;[1 1 1] this doesnt include waves:(
  (Rendering|Debug|DrawDebugSphere AtLocation 1e+02 12 "(R=1.000000,G=1.000000,B=1.000000,A=1.000000)" 0.0)
  (Rendering|Debug|DrawDebugSphere _outwatersurfacelocation 1e+02 12 "(R=1.000000,G=0.043423,B=0.866597,A=1.000000)" 0.0)
  (return _outwatersurfacelocation))

(fn GetWaterBottomLocation
  (params (AtLocation :type Vector :default "0, 0, 0"))
  (bind _waterbodybp (Variables|Default|GetWaterBodyBP))
  (bind _waterbodycomponent (Variables|/Script/Water.WaterBody|GetWaterBodyComponent _waterbodybp))
  (bind (_outwatersurfacelocation _outwatersurfacenormal _outwatervelocity _outwaterdepth) (WaterBody|GetWaterSurfaceInfoatLocation _waterbodycomponent AtLocation true))
  (return (- _outwatersurfacelocation (Math|Vector|MakeVector 0.0 0.0 _outwaterdepth))))