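; Throw prediction actor that previews the arc and landing point of a thrown object while enabled.
; Enabling creates a spline and a hidden end-point marker actor; disabling destroys both along with the spline meshes.
; Each tick it predicts the projectile path from the supplied start and velocity, feeds it into the spline, and places the marker at any impact.
; Spline meshes are destroyed and rebuilt every tick in fixed-length segments.
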(event EventBeginPlay)

(event Collision|EventActorBeginOverlap
  (params (OtherActor :type Actor%20Object%20Reference)))

(event EventTick
  (params (DeltaSeconds :type Float%20%28single-precision%29))
  (if (Variables|Default|GetIsEnabled)
    (CallFunction|DrawPredictionSpline)))

(fn ConstructionScript)

(fn CreatePredictionSpline
  (bind _returnvalue (AddComponent|AddSplineComponent false))
  (Variables|Default|SetPredictionSpline _returnvalue)
  (bind _returnvalue_2 (Game|SpawnActorfromClass "/Game/Blueprints/ThrowableObject/BP_PredictionEndPoint.BP_PredictionEndPoint_C" (Math|Transform|MakeTransform "0, 0, 0" "0, 0, 0" "1.000000,1.000000,1.000000") "Undefined" 0 0))
  (bind _output_get (Variables|Default|SetPredictionEndPoint _returnvalue_2))
  (Rendering|SetActorHiddenInGame _output_get true))

(fn DestroyPredictionSpline
  (bind _predictionspline (Variables|Default|GetPredictionSpline)
    (:then
      (Components|DestroyComponent _predictionspline)
      (Variables|Default|SetPredictionSpline 0)
      (CallFunction|DestroyPredictionMeshes)
      (Actor|DestroyActor (Variables|Default|GetPredictionEndPoint))
      (Variables|Default|SetPredictionEndPoint 0))
    (:else)))

(fn DestroyPredictionMeshes
  (for _array_element (Variables|Default|GetPredictionSplineMeshes)
    (Components|DestroyComponent _array_element))
  (Utilities|Array|Clear (Variables|Default|GetPredictionSplineMeshes)))

(fn DrawPredictionSpline
  (bind _predictionendpoint (Variables|Default|GetPredictionEndPoint))
  (Utilities|IsPredictionSplineValid
    (:Is%20Valid
      (Utilities|FlowControl|Sequence
        (:then_0
          (bind (_outhit _outpathpositions _outlasttracedestination _returnvalue) (Class|GameplayStatics|BlueprintPredictProjectilePathbyTraceChannel (Variables|Default|GetThrowStartPos) (Variables|Default|GetThrowVelocity) true 25.0 "ECC_WorldDynamic" false 0 "None"))
          (if _returnvalue
            (Rendering|SetActorHiddenInGame _predictionendpoint false)
            (Transformation|SetActorLocation (Variables|Default|GetPredictionEndPoint) (.ImpactPoint (Collision|BreakHitResult _outhit)) false true)
            (else
              (Rendering|SetActorHiddenInGame _predictionendpoint true)))
          (Spline|SetSplinePoints (Variables|Default|GetPredictionSpline) _outpathpositions "World" true)
          (CallFunction|DestroyPredictionMeshes))
        (:then_1
          (for _index (range 0 (Math|Float|Truncate (/ (Spline|GetSplineLength (Variables|Default|GetPredictionSpline)) 1e+02)))
            (LocalVariables|SetIndex _index)
            (bind _returnvalue_2 (AddComponent|AddSplineMeshComponent true))
            (Utilities|Array|Add (Variables|Default|GetPredictionSplineMeshes) _returnvalue_2)
            (SplineMesh|SetStartandEnd _returnvalue_2 (Spline|GetLocationatDistanceAlongSpline (Variables|Default|GetPredictionSpline) (Math|Conversions|ToFloat(Integer) (* (LocalVariables|GetIndex) 100)) "World") (Math|Vector|ClampVectorSize (Spline|GetTangentatDistanceAlongSpline (Variables|Default|GetPredictionSpline) (Math|Conversions|ToFloat(Integer) (* (LocalVariables|GetIndex) 100)) "World") 0.0 1e+02) (Spline|GetLocationatDistanceAlongSpline (Variables|Default|GetPredictionSpline) (Math|Conversions|ToFloat(Integer) (* (+ (LocalVariables|GetIndex) 1) 100)) "World") (Math|Vector|ClampVectorSize (Spline|GetTangentatDistanceAlongSpline (Variables|Default|GetPredictionSpline) (Math|Conversions|ToFloat(Integer) (* (+ (LocalVariables|GetIndex) 1) 100)) "World") 0.0 1e+02) true :!class /Script/Engine.SplineMeshComponent)))))))

(fn SetEnabled
  (params (enabled :type Boolean))
  (bind _output_get (Variables|Default|SetIsEnabled enabled))
  (Development|PrintString (Utilities|String|Append "prediction enabled " (Utilities|String|ToString(Boolean) _output_get)))
  (if _output_get
    (CallFunction|CreatePredictionSpline)
    (else
      (CallFunction|DestroyPredictionSpline))))

(fn UpdateValues
  (params (start :type Vector) (velocity :type Vector))
  (Variables|Default|SetThrowStartPos start)
  (Variables|Default|SetThrowVelocity velocity))