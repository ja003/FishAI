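; BP_CPP_MyCharacterZorg is a player character Blueprint with third-person camera controls and a throwing ability.
; Camera input rotates the spring arm and steps its arm length in or out, while a direct camera pitch call is disabled.
; Throwing starts through a Throwing component only when the character is not swimming and that component allows it.
; While throwing or while a spawned object exists, aim input yaws the capsule to turn the character.
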(fn ConstructionScript)

(fn UpdateCameraRotation
  (params (deltaX :type Float%20%28double-precision%29) (deltaY :type Float%20%28double-precision%29))
  (Transformation|AddRelativeRotation (Variables|Camera|GetCamera) (Math|Rotator|MakeRotator 0.0 deltaY 0.0) false false)
  (Transformation|AddRelativeRotation (Variables|Camera|GetSpringArm) (Math|Rotator|MakeRotator 0.0 deltaY (* deltaX 3.0)) false false))

(fn UpdateCameraDistance
  (params (increase :type Boolean))
  (bind _springarm (Variables|Camera|GetSpringArm))
  (Variables|/Script/Engine.SpringArmComponent|SetTargetArmLength _springarm (+ (Variables|/Script/Engine.SpringArmComponent|GetTargetArmLength _springarm) (* 1.5e+02 (Math|Float|SelectFloat 1.0 -1.0 increase)))))

(fn StartThrowing
  (bind _throwing (Variables|Default|GetThrowing))
  (if (and (not (AI|Components|NavMovement|IsSwimming (Variables|Character|GetCharacterMovement) :!class /Script/Engine.NavMovementComponent)) (Class|Throwing|CanStartThrowing _throwing))
    (Class|Throwing|SetIsThrowing _throwing true)))

(fn UpdateAim
  (params (RotationX :type Float%20%28double-precision%29))
  (bind _throwing (Variables|Default|GetThrowing))
  (if (or (Utilities|IsValid (Variables|/Script/FishAi.Throwing|GetSpawnedObject _throwing)) (Variables|/Script/FishAi.Throwing|GetbIsThrowing _throwing))
    (Transformation|AddRelativeRotation (Variables|Default|GetCapsuleComponent) (Math|Rotator|MakeRotator 0.0 0.0 (* RotationX 2.5)) false false)))