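; BP_Water is a test actor that probes cursor and overlap detection on a referenced LakeBody water actor.
; BeginPlay binds handlers to the lake's cursor-over and actor-overlap events, which print debug text; the overlap handler prints the overlapped actor's name, not the other actor's.
; Tick prints the count of actors overlapping the lake every frame.
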(event Custom|CustomEvent
  (params (TouchedActor :type Actor%20Object%20Reference))
  (Development|PrintString "cursor"))

(event Custom|Overlap
  (params (OverlappedActor :type Actor%20Object%20Reference) (OtherActor :type Actor%20Object%20Reference))
  (Development|PrintString (Utilities|GetDisplayName OverlappedActor)))

(event EventTick
  (params (DeltaSeconds :type Float%20%28single-precision%29))
  (Development|PrintString (Utilities|String|ToString(Integer) (Utilities|Array|Length (Collision|GetOverlappingActors (Variables|Default|GetLakeBody) 0 :!class /Script/Engine.Actor)))))

(event EventBeginPlay
  (bind _lakebody (Variables|Default|GetLakeBody))
  (EventDispatchers|BindEventtoOnBeginCursorOver _lakebody (delegate Custom|CustomEvent))
  (Collision|BindEventtoOnActorBeginOverlap _lakebody (delegate Custom|Overlap)))

(fn ConstructionScript)