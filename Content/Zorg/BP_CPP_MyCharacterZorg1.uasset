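; Player character Blueprint for Zorg, handling object throwing with trajectory preview, camera rotation and zoom, and swimming.
; Input sets a throwing flag and adjusts throw power, while Tick feeds the launch point and velocity to the level's BP_ThrowPrediction actor.
; Throw launches and releases the held object, but the rock spawn-and-attach logic is disconnected and nothing here calls Throw.
; Water body overlaps switch movement between Swimming and Walking and toggle the physics volume's water flag.
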(event Input|EnhancedActionEvents|EnhancedInputActionIA_Throw
  (params (ActionValue :type Boolean) (ElapsedSeconds :type Float%20%28double-precision%29) (TriggeredSeconds :type Float%20%28double-precision%29) (InputAction :type Input%20Action%20Object%20Reference :default "/Game/Input/Actions/IA_Throw.IA_Throw"))
  (:Triggered
    (Variables|Default|GetSpawnedThrowableObject
      (:then
        (Variables|Default|SetIsThrowing true)
        (Development|PrintString "start throwing"))
      (:else))))

(event Input|EnhancedActionEvents|EnhancedInputActionIA_DeselectObject
  (params (ActionValue :type Boolean) (ElapsedSeconds :type Float%20%28double-precision%29) (TriggeredSeconds :type Float%20%28double-precision%29) (InputAction :type Input%20Action%20Object%20Reference :default "/Game/Input/Actions/IA_DeselectObject.IA_DeselectObject"))
  (:Triggered
    (Default|SetEnabled (Variables|Default|GetThrowPrediction) false)))

(event Input|EnhancedActionEvents|EnhancedInputActionIA_UpdateThrowPower
  (params (ActionValue :type Float%20%28double-precision%29) (ElapsedSeconds :type Float%20%28double-precision%29) (TriggeredSeconds :type Float%20%28double-precision%29) (InputAction :type Input%20Action%20Object%20Reference :default "/Game/Input/Actions/IA_UpdateThrowPower.IA_UpdateThrowPower"))
  (:Triggered
    (Variables|Default|SetThrowPower (+ (Variables|Default|GetThrowPower) (* ActionValue 5e+01)))))

(event EventTick
  (params (DeltaSeconds :type Float%20%28single-precision%29))
  (|UpdateThrowPrediction))

(event EventBeginPlay
  (bind _returnvalue (Actor|GetActorOfClass "/Game/Blueprints/ThrowableObject/BP_ThrowPrediction.BP_ThrowPrediction_C"))
  (Variables|Default|SetThrowPrediction _returnvalue))

(fn ConstructionScript)

(fn Throw
  (Variables|Default|GetSpawnedThrowableObject
    (:then
      (Development|PrintString "throw")
      (Class|ThrowableObject|SetVelocity (Variables|Default|GetSpawnedThrowableObject) (* (Math|Vector|GetForwardVector (Variables|Default|GetThrowStart)) (Variables|Default|GetThrowPower)))
      (Variables|Default|SetSpawnedThrowableObject 0))
    (:else)))

(fn UpdateCameraRotation
  (params (deltaX :type Float%20%28double-precision%29) (deltaY :type Float%20%28double-precision%29))
  (Transformation|AddRelativeRotation (Variables|Camera|GetCamera) (Math|Rotator|MakeRotator 0.0 deltaY 0.0) false false)
  (Transformation|AddRelativeRotation (Variables|Camera|GetSpringArm) (Math|Rotator|MakeRotator 0.0 0.0 (* deltaX 3.0)) false false))

(fn UpdateCameraDistance
  (params (increase :type Boolean))
  (bind _springarm (Variables|Camera|GetSpringArm))
  (Variables|/Script/Engine.SpringArmComponent|SetTargetArmLength _springarm (+ (Variables|/Script/Engine.SpringArmComponent|GetTargetArmLength _springarm) (* 1.5e+02 (Math|Float|SelectFloat 1.0 -1.0 increase)))))