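; Player character Blueprint that handles throw input and drives a throw trajectory preview.
; On BeginPlay it caches the level's BP_ThrowPrediction actor, which weapon select and deselect inputs switch on and off.
; While enabled, Tick feeds it the ThrowStart location and a hardcoded velocity, leaving a forward-vector times ThrowPower calculation unused.
; Throwing itself is a stub: the input only sets IsThrowing and prints, and the Throw function just prints.
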(event Input|EnhancedActionEvents|EnhancedInputActionIA_Throw
  (params (ActionValue :type Boolean) (ElapsedSeconds :type Float%20%28double-precision%29) (TriggeredSeconds :type Float%20%28double-precision%29) (InputAction :type Input%20Action%20Object%20Reference :default "/Game/TopDown/Input/Actions/IA_Throw.IA_Throw"))
  (:Triggered
    (Variables|Default|SetIsThrowing true)
    (Development|PrintString "throw")))

(event Input|EnhancedActionEvents|EnhancedInputActionIA_SelectWeapon1
  (params (ActionValue :type Boolean) (ElapsedSeconds :type Float%20%28double-precision%29) (TriggeredSeconds :type Float%20%28double-precision%29) (InputAction :type Input%20Action%20Object%20Reference :default "/Game/TopDown/Input/Actions/IA_SelectWeapon1.IA_SelectWeapon1"))
  (:Triggered
    (Default|SetEnabled (Variables|Default|GetThrowPrediction) true)
    (Development|PrintString "weapon")))

(event Input|EnhancedActionEvents|EnhancedInputActionIA_DeselectWeapon
  (params (ActionValue :type Boolean) (ElapsedSeconds :type Float%20%28double-precision%29) (TriggeredSeconds :type Float%20%28double-precision%29) (InputAction :type Input%20Action%20Object%20Reference :default "/Game/TopDown/Input/Actions/IA_DeselectWeapon.IA_DeselectWeapon"))
  (:Triggered
    (Default|SetEnabled (Variables|Default|GetThrowPrediction) false)))

(event EventTick
  (params (DeltaSeconds :type Float%20%28single-precision%29))
  (bind _throwprediction (Variables|Default|GetThrowPrediction))
  (if (Variables|/Game/Blueprints/ThrowableObject/BP_ThrowPrediction.BP_ThrowPrediction_C|GetIsEnabled _throwprediction)
    (Default|UpdateValues _throwprediction (Transformation|GetWorldLocation (Variables|Default|GetThrowStart)) "1000.000000,0.000000,1000.000000")))

(event EventBeginPlay
  (bind _returnvalue (Actor|GetActorOfClass "/Game/Blueprints/ThrowableObject/BP_ThrowPrediction.BP_ThrowPrediction_C"))
  (Variables|Default|SetThrowPrediction _returnvalue))

(fn ConstructionScript)

(fn Throw
  (Development|PrintString "throw"))